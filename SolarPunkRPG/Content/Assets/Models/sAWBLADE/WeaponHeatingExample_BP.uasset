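; Example sawblade actor that previews a heated-metal material effect on its blade mesh.
; The construction script pushes heat amount, heat radius and coloration radius variables into scalar material parameters on the blade.
; It also sets a world-space Offset vector from the root location plus a heat center offset, positioning the heat center.
; The event graph has no runtime logic, so values update only when construction reruns.
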(event `self.ReceiveBeginPlay`)

(fn `UserConstructionScript`
  (bind _pvcblade_low (`self.PVCblade_low`))
  (`MeshComponent.SetScalarParameterValueOnMaterials` _pvcblade_low "Heat" (`self.Blade_Heat`))
  (`MeshComponent.SetScalarParameterValueOnMaterials` _pvcblade_low "Heat_Radius" (`self.Blade_HeatRadius`))
  (`MeshComponent.SetScalarParameterValueOnMaterials` _pvcblade_low "Coloration_Radius" (`self.Blade_ColorationRadius`))
  (`MeshComponent.SetVectorParameterValueOnMaterials` _pvcblade_low "Offset" (+ (`SceneComponent.K2_GetComponentLocation` (`self.DefaultSceneRoot`)) (`self.HeatCenter_Offset`))))