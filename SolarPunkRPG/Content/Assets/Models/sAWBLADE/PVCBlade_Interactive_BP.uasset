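; Interactive saw blade actor that shows a sparking, heating and cooling effect, played automatically on a timed sequence after BeginPlay.
; BeginHeating activates two Niagara spark systems, then a timeline drives the blade material's heat, heat radius and coloration radius parameters.
; CoolDown later lowers or animates only the heat through a second timeline, so coloration and radius remain.
; The construction script seeds these parameters and sets the heat center from world location plus an offset.
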(event `Begin Heating`
  (bind _pvcblade_low (`self.PVCblade_low`))
  (`ActorComponent.Activate` (`self.Electric_Sparks_NS`) false)
  (`ActorComponent.Activate` (`self.Electric_Sparks_NS1`) false)
  (`KismetSystemLibrary.Delay` 1.0)
  (`TimelineComponent.SetPlayRate` (`self.Heating`) 2.0)
  (bind (_direction _coloring _heat_radius _heat) (`Timeline|Heating`)
    (:`Update`
      (bind _output_get (set `self.Blade_Coloration` (`KismetMathLibrary.Lerp` 0.0 45.0 _coloring)))
      (`MeshComponent.SetScalarParameterValueOnMaterials` _pvcblade_low "Coloration_Radius" _output_get)
      (bind _output_get_2 (set `self.Blade_HeatRadius` (`KismetMathLibrary.Lerp` 0.0 27.0 _heat_radius)))
      (`MeshComponent.SetScalarParameterValueOnMaterials` _pvcblade_low "Heat_Radius" _output_get_2)
      (bind _output_get_3 (set `self.Blade_Heat` (`KismetMathLibrary.Lerp` 0.0 10.0 _heat)))
      (`MeshComponent.SetScalarParameterValueOnMaterials` _pvcblade_low "Heat" _output_get_3))))

(event `self.ReceiveBeginPlay`
  (`KismetSystemLibrary.Delay` 2.0)
  (`self.Begin Heating`)
  (`KismetSystemLibrary.Delay` 10.0)
  (`self.Cool Down`))

(event `Cool Down`
  (`TimelineComponent.SetPlayRate` (`self.Cooling`) 4.0)
  (bind (_direction _heat) (`Timeline|Cooling` :!via `PlayFromStart`)
    (:`Update`
      (bind _output_get (set `self.Blade_Heat` (`KismetMathLibrary.Lerp` 0.0 10.0 _heat)))
      (`MeshComponent.SetScalarParameterValueOnMaterials` (`self.PVCblade_low`) "Heat" _output_get))))

(fn `UserConstructionScript`
  (bind _pvcblade_low (`self.PVCblade_low`))
  (`MeshComponent.SetScalarParameterValueOnMaterials` _pvcblade_low "Heat" (`self.Blade_Heat`))
  (`MeshComponent.SetScalarParameterValueOnMaterials` _pvcblade_low "Heat_Radius" (`self.Blade_HeatRadius`))
  (`MeshComponent.SetScalarParameterValueOnMaterials` _pvcblade_low "Coloration_Radius" (`self.Blade_Coloration`))
  (`MeshComponent.SetVectorParameterValueOnMaterials` _pvcblade_low "Offset" (+ (`SceneComponent.K2_GetComponentLocation` (`self.DefaultSceneRoot`)) (`self.HeatCenter_Offset`))))